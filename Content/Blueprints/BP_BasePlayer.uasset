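; BP_BasePlayer is a player character Blueprint drafted for Enhanced Input movement, look and jump, but none of its logic is connected.
; BeginPlay, IA_Move and IA_Look are empty, and no IA_Jump event exists.
; Unreached nodes would add the IMC_BasePlayerController mapping context, apply yaw and pitch, jump, and move along actor right and a forward vector from zero rotation.
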(event `self.ReceiveBeginPlay`
  ; Add input controls
)

(event `EnhancedInput|/Game/Inputs/BaseMagicCharacter/IA_Move`
  (params (ActionValue :type "Vector2D Structure") (ElapsedSeconds :type "Float (double-precision)") (TriggeredSeconds :type "Float (double-precision)") (InputAction :type "InputAction Object Reference" :default "/Game/Inputs/BaseMagicCharacter/IA_Move.IA_Move"))
  ; Add IA_Move
)

(event `EnhancedInput|/Game/Inputs/BaseMagicCharacter/IA_Jump`
  (params (ActionValue :type Boolean) (ElapsedSeconds :type "Float (double-precision)") (TriggeredSeconds :type "Float (double-precision)") (InputAction :type "InputAction Object Reference" :default "/Game/Inputs/BaseMagicCharacter/IA_Jump.IA_Jump"))
  ; Add IA_Jump
)

(event `EnhancedInput|/Game/Inputs/BaseMagicCharacter/IA_Look`
  (params (ActionValue :type "Vector2D Structure") (ElapsedSeconds :type "Float (double-precision)") (TriggeredSeconds :type "Float (double-precision)") (InputAction :type "InputAction Object Reference" :default "/Game/Inputs/BaseMagicCharacter/IA_Look.IA_Look"))
  ; Add IA_Look
)

(fn `UserConstructionScript`)